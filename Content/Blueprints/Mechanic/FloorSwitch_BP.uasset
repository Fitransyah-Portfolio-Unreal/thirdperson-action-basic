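; FloorSwitch_BP is a floor switch that animates its pressure plate and a door up and down.
; Raise and lower events play or reverse two timelines, one for the door and one for the switch.
; Each timeline update passes its elevation to UpdateDoorLocation or UpdateFloorSwitchLocation, which are defined outside this graph, as are the triggers.
; An unconnected node that offsets the door upward never runs.
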(event `self.RaiseDoor`
  (bind (_direction _doorelevation) (`Timeline|DoorTimeline` :`NewTime` (`GameplayStatics.GetWorldDeltaSeconds`) :!label _label)
    (:`Update`
      (`self.UpdateDoorLocation` _doorelevation))))

(event `self.LowerDoor`
  (goto _label :!via `Reverse`))

(event `self.LowerFloorSwitch`
  (bind (_direction _floorswithelevation) (`Timeline|FloorSwitchTimeline` :`NewTime` (`GameplayStatics.GetWorldDeltaSeconds`) :!label _label_2)
    (:`Update`
      (`self.UpdateFloorSwitchLocation` _floorswithelevation))))

(event `self.RaiseFloorSwitch`
  (goto _label_2 :!via `Reverse`))

(fn `UserConstructionScript`)